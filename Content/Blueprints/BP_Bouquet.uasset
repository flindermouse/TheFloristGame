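; BP_Bouquet is an actor that manages an editable, priced bouquet of BP_Flower actors.
; It spawns and removes flowers, tracks a glowing active one, and applies type or colour changes to it or the whole bouquet.
; Edits recompute the price as the sum of the flowers' prices.
; UpdatePositions is called on add and remove but is empty, leaving its fan-out layout logic disconnected.
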(fn `AddNewFlower`
  (params (newFlowType :type Name) (newFlowCol :type Name))
  (bind _returnvalue (`|SpawnActorFromClass` "/Game/Blueprints/BP_Flower.BP_Flower_C" (`KismetMathLibrary.MakeTransform` (`self.startLoc`)) "Undefined" "OverrideRootScale" self null))
  (bind _returnvalue_2 (`KismetArrayLibrary.Array_Add` (`self.flowers`) _returnvalue))
  (`self.SetActiveFlower` _returnvalue_2)
  (`self.SetAFType` newFlowType)
  (`self.SetAFColour` newFlowCol)
  (`self.SetPrice`)
  (`self.UpdatePositions`))

(fn `RemoveActiveFlower`
  (locals (toDestroy :type "/Game/Blueprints/BP_Flower Object Reference"))
  (bind _flowers (`self.flowers`))
  (bind _activeindex (`self.activeIndex`))
  (set `local.toDestroy` (`|GetArrayItem` _flowers _activeindex))
  (`KismetArrayLibrary.Array_Remove` _flowers _activeindex)
  (if (!= (`self.activeIndex`) 0)
    (`self.SetActiveFlower` (- (`self.activeIndex`) 1))
    (else
      (`self.SetActiveFlower` (- (`KismetArrayLibrary.Array_Length` (`self.flowers`)) 1))))
  (`self.K2_DestroyActor` (`local.toDestroy`))
  (`self.SetPrice`)
  (`self.UpdatePositions`))

(fn `SetActiveFlower`
  (params (newActiveInd :type Integer))
  (`/Game/Blueprints/BP_Flower.SetGlow` (`|GetArrayItem` (`self.flowers`) (`self.activeIndex`)) false)
  (bind _output_get (set `self.activeIndex` newActiveInd))
  (`/Game/Blueprints/BP_Flower.SetGlow` (`|GetArrayItem` (`self.flowers`) _output_get) true))

(fn `SetAFColour`
  (params (colour :type Name))
  (`/Game/Blueprints/BP_Flower.SetMeshColour` (`|GetArrayItem` (`self.flowers`) (`self.activeIndex`)) colour)
  (`self.SetPrice`))

(fn `SetAFType`
  (params (type :type Name))
  (`/Game/Blueprints/BP_Flower.SetMesh` (`|GetArrayItem` (`self.flowers`) (`self.activeIndex`)) type)
  (`self.SetPrice`))

(fn `SetAllColour`
  (params (colour :type Name))
  (for _array_element (`self.flowers`)
    (`/Game/Blueprints/BP_Flower.SetMeshColour` _array_element colour))
  (`self.SetPrice`))

(fn `SetAllType`
  (params (type :type Name))
  (for _array_element (`self.flowers`)
    (`/Game/Blueprints/BP_Flower.SetMesh` _array_element type))
  (`self.SetPrice`))

(fn `SetPrice`
  (set `self.currentPrice` 0.0)
  (for _array_element (`self.flowers`)
    (set `self.currentPrice` (+ (`/Game/Blueprints/BP_Flower.currentPrice` _array_element) (`self.currentPrice`)))))

(fn `UpdatePositions`
  (locals (mid :type Integer) (locChangeR :type "Vector Structure") (rotChangeR :type "Vector Structure") (locChangeL :type "Vector Structure") (rotChangeL :type "Vector Structure") (currentFlower :type "/Game/Blueprints/BP_Flower Object Reference")))

(fn `UserConstructionScript`)