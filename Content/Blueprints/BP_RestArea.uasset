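; BP_RestArea is a limited-use rest spot that fully restores the player's health and ability power.
; Its box overlap tracks the player and shows a UI_RestOverlay widget while uses remain.
; RestoreHealthStamina, not called within this file, refills both components, spends a use, spawns the NS_HolyAEO effect and hides the overlay.
; It also saves the remaining uses per level name to the Florinstance game instance.
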(event `self.ReceiveBeginPlay`
  (bind _returnvalue (`|CreateWidget` "/Game/Blueprints/UI_RestOverlay.UI_RestOverlay_C"))
  (set `self.text` _returnvalue))

(event `self.Box.OnComponentBeginOverlap`
  (params (OverlappedComponent :type "PrimitiveComponent Object Reference") (OtherActor :type "Actor Object Reference") (OtherComp :type "PrimitiveComponent Object Reference") (OtherBodyIndex :type Integer) (bFromSweep :type Boolean) (SweepResult :type "HitResult Structure (by ref)"))
  (if (== OtherActor (`GameplayStatics.GetPlayerCharacter` 0))
    (set `self.inArea` true)
    (if (> (`self.numUses`) 0)
      (`UserWidget.AddToViewport` (`self.text`) 0)
      (set `self.overlapActor` OtherActor))))

(event `self.Box.OnComponentEndOverlap`
  (params (OverlappedComponent :type "PrimitiveComponent Object Reference") (OtherActor :type "Actor Object Reference") (OtherComp :type "PrimitiveComponent Object Reference") (OtherBodyIndex :type Integer))
  (if (== OtherActor (`GameplayStatics.GetPlayerCharacter` 0))
    (set `self.inArea` false)
    (`Widget.RemoveFromParent` (`self.text`))
    (set `self.overlapActor` null)))

(fn `GetNumUses`
  (returns (uses :type Integer))
  (return (`self.numUses`)))

(fn `PlayerInArea`
  (returns (in :type Boolean))
  (return (`self.inArea`)))

(fn `RestoreHealthStamina`
  (bind _returnvalue (`GameplayStatics.GetPlayerCharacter` 0))
  (bind (_returnvalue_location _returnvalue_rotation) (`KismetMathLibrary.BreakTransform` (`self.GetTransform` _returnvalue)))
  (if (> (`self.numUses`) 0)
    (if (== (`self.overlapActor`) _returnvalue)
      (bind _asbp_florist_character (cast `/Game/ThirdPerson/Blueprints/BP_FloristCharacter` _returnvalue))
      (bind _returnvalue_2 (`TheFloristCharacter.GetHealthComponent` _asbp_florist_character))
      (`HealthStatusComponent.Heal` _returnvalue_2 (`HealthStatusComponent.GetMaxHealth` _returnvalue_2))
      (bind _returnvalue_3 (`TheFloristCharacter.GetAbilityComponent` _asbp_florist_character))
      (`AbilityComponent.SetCurrentPower` _returnvalue_3 (`AbilityComponent.GetMaxPower` _returnvalue_3))
      (bind _output_get (set `self.numUses` (- (`self.numUses`) 1)))
      (bind _asflorinstance (cast `/Game/Blueprints/Florinstance` (`GameplayStatics.GetGameInstance`))
        (:`then`
          (bind _returnvalue_4 (`GameplayStatics.GetCurrentLevelName` true))
          (`/Game/Blueprints/Florinstance.SetRestUses` _asflorinstance _returnvalue_4 _output_get))
        (:`CastFailed`
          _))
      (`NiagaraFunctionLibrary.SpawnSystemAtLocation` "/Game/AEO_Abilities/MagicAEO_Optimal/Niagara/Holy/NS_HolyAEO.NS_HolyAEO" _returnvalue_location _returnvalue_rotation)
      (`Widget.RemoveFromParent` (`self.text`)))))

(fn `SetNumUses`
  (params (uses :type Integer))
  (set `self.numUses` uses))

(fn `UserConstructionScript`)