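; BP_Flower is a flower whose type, colour, price and glow can be changed at runtime.
; Type and colour names look up meshes and materials in maps, with tulips using swapped material slots for petal colour and greenery.
; Each change recomputes the price as the sum of the type and colour prices.
; SetGlow switches a point light on or off through its intensity.
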(fn `SetGlow`
  (params (turnOn :type Boolean))
  (if turnOn
    (`LightComponent.SetIntensity` (`self.PointLight`) 1000.0)
    (else
      (`LightComponent.SetIntensity` (`self.PointLight`) 0.0))))

(fn `SetMesh`
  (params (typeName :type Name))
  (bind _value (`BlueprintMapLibrary.Map_Find` (`self.flowCol`) (`self.currentColour`)))
  (bind _output_get (set `self.currentType` typeName))
  (`StaticMeshComponent.SetStaticMesh` (`self.CurrentMesh`) (`BlueprintMapLibrary.Map_Find` (`self.flowMesh`) _output_get))
  (if (== (`self.currentType`) "Tulip")
    (`PrimitiveComponent.SetMaterial` (`self.CurrentMesh`) 0 "/Game/StarterContent/Materials/M_Ground_Grass.M_Ground_Grass")
    (`PrimitiveComponent.SetMaterial` (`self.CurrentMesh`) 1 _value)
    (else
      (`PrimitiveComponent.SetMaterial` (`self.CurrentMesh`) 1 "/Game/StarterContent/Materials/M_Ground_Moss.M_Ground_Moss")
      (`PrimitiveComponent.SetMaterial` (`self.CurrentMesh`) 0 _value)
      (`SceneComponent.SetWorldScale3D` (`self.CurrentMesh`) (0.8 0.8 0.8))))
  (`self.SetPrice`))

(fn `SetMeshColour`
  (params (colName :type Name))
  (locals (newColour :type "MaterialInterface Object Reference"))
  (bind _newcolour (`local.newColour`))
  (bind _output_get (set `self.currentColour` colName))
  (set `local.newColour` (`BlueprintMapLibrary.Map_Find` (`self.flowCol`) _output_get))
  (if (== (`self.currentType`) "Tulip")
    (`PrimitiveComponent.SetMaterial` (`self.CurrentMesh`) 1 _newcolour)
    (else
      (`PrimitiveComponent.SetMaterial` (`self.CurrentMesh`) 0 _newcolour)))
  (`self.SetPrice`)
  (`SceneComponent.SetWorldScale3D` (`self.CurrentMesh`) (0.8 0.8 0.8)))

(fn `SetPrice`
  (set `self.currentPrice` (+ (`BlueprintMapLibrary.Map_Find` (`self.flowPrice`) (`self.currentType`)) (`BlueprintMapLibrary.Map_Find` (`self.colPrice`) (`self.currentColour`)))))

(fn `UserConstructionScript`)