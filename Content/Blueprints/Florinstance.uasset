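; Florinstance appears to be the game instance that carries player state between overworld levels and turn-based combat.
; Separate setters and getters cache health, power, abilities and items, with flags marking whether each pawn's data is saved.
; ChangeLevel saves the overworld pawn before opening a level, also storing a return transform for TurnBasedTest.
; It also records removed monsters' start locations and per-level rest uses, and merges combat rewards into items.
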(fn `AddCombatRewards`
  (locals (amount :type Integer))
  (bind _pitems (`self.pItems`))
  (for _array_element (`self.lastRewards`)
    (if (`BlueprintMapLibrary.Map_Contains` _pitems _array_element)
      (bind _output_get (set `local.amount` (`BlueprintMapLibrary.Map_Find` _pitems _array_element)))
      (`BlueprintMapLibrary.Map_Add` _pitems _array_element (+ _output_get 1))
      (else
        (`BlueprintMapLibrary.Map_Add` _pitems _array_element 1)))))

(fn `ChangeLevel`
  (params (player :type "Actor Object Reference") (level :type Name))
  (bind _returnvalue (`GameplayStatics.GetCurrentLevelName` true))
  (set `self.lastLevelName` _returnvalue)
  (if (== level "TurnBasedTest")
    (`self.SetReturnPoint`))
  (bind _asbp_florist_character (cast `/Game/ThirdPerson/Blueprints/BP_FloristCharacter` player))
  (`self.SetOverworldPawn` (`/Game/ThirdPerson/Blueprints/BP_FloristCharacter.PlayerInventory` _asbp_florist_character) (`/Game/ThirdPerson/Blueprints/BP_FloristCharacter.HealthStatus` _asbp_florist_character) (`/Game/ThirdPerson/Blueprints/BP_FloristCharacter.Ability` _asbp_florist_character))
  (`GameplayStatics.OpenLevel` level))

(fn `GetOverworldPawn`
  (returns (pInv :type "Map of Item Object Reference to Integer") (pHealth :type "Array of Float (double-precision)") (pAbils :type "Array of Ability Object Reference") (pPow :type "Array of Float (double-precision)") (pMaxC :type Integer))
  (return (`self.pItems`) (`self.playerHealth`) (`self.pAbilities`) (`self.playerPower`) (`self.pMaxCapac`)))

(fn `GetRestUses`
  (params (level :type String))
  (returns (uses :type Integer))
  (return (`BlueprintMapLibrary.Map_Find` (`self.levelRestUses`) level)))

(fn `GetTBPawn`
  (returns (playH :type "Array of Float (double-precision)") (playA :type "Array of Ability Object Reference") (playP :type "Array of Float (double-precision)") (playC :type Integer))
  (return (`self.playerHealth`) (`self.pAbilities`) (`self.playerPower`) (`self.pMaxCapac`)))

(fn `HasOverworldPawn`
  (returns (haspawn :type Boolean))
  (return (`self.oPawn`)))

(fn `HasRestUses`
  (params (levelName :type String))
  (returns (hasUsesStored :type Boolean))
  (return (`BlueprintMapLibrary.Map_Contains` (`self.levelRestUses`) levelName)))

(fn `HasTBPawn`
  (returns (has :type Boolean))
  (return (`self.tbPawn`)))

(fn `RemoveWanderingMonster`
  (params (monst :type "/Game/ThirdPerson/Blueprints/BP_WanderingMonster Object Reference"))
  (`KismetArrayLibrary.Array_Add` (`self.monstStartLocs`) (`/Game/ThirdPerson/Blueprints/BP_WanderingMonster.startLoc` monst)))

(fn `SetOverworldPawn`
  (params (pInv :type "PlayerInventory Object Reference") (pHealth :type "HealthStatusComponent Object Reference") (pAbil :type "AbilityComponent Object Reference"))
  (set `self.pItems` (`PlayerInventory.GetItemMap` pInv))
  (`KismetArrayLibrary.Array_Set` (`self.playerHealth`) 0 (`HealthStatusComponent.GetCurrentHealth` pHealth))
  (`KismetArrayLibrary.Array_Set` (`self.playerPower`) 0 (`AbilityComponent.GetCurrentPower` pAbil))
  (set `self.oPawn` true))

(fn `SetRestUses`
  (params (levelName :type String) (uses :type Integer))
  (`BlueprintMapLibrary.Map_Add` (`self.levelRestUses`) levelName uses))

(fn `SetReturnPoint`
  (set `self.return` (`Actor.GetTransform` (`GameplayStatics.GetPlayerPawn` 0))))

(fn `SetTBPawn`
  (params (hc :type "HealthStatusComponent Object Reference") (ac :type "AbilityComponent Object Reference"))
  (bind _playerhealth (`self.playerHealth`))
  (bind _playerpower (`self.playerPower`))
  (`KismetArrayLibrary.Array_Set` _playerhealth 0 (`HealthStatusComponent.GetCurrentHealth` hc) true)
  (`KismetArrayLibrary.Array_Set` _playerhealth 1 (`HealthStatusComponent.GetMaxHealth` hc) true)
  (set `self.pAbilities` (`AbilityComponent.GetAbilityArray` ac))
  (set `self.pMaxCapac` (`AbilityComponent.GetMaxCapacity` ac))
  (`KismetArrayLibrary.Array_Set` _playerpower 0 (`AbilityComponent.GetCurrentPower` ac) true)
  (`KismetArrayLibrary.Array_Set` _playerpower 1 (`AbilityComponent.GetMaxPower` ac) true)
  (`KismetArrayLibrary.Array_Set` _playerpower 2 (`AbilityComponent.GetPowerRegenRate` ac) true)
  (set `self.tbPawn` true))