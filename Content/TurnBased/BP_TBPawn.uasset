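; Turn-based pawn that carries health and ability state over from the Florinstance game instance.
; On BeginPlay it adds four temporary test abilities to its Ability component, then looks for a stored pawn.
; If one exists, RestorePawn copies health into HealthStatus and sets the ability array, power, regen rate and capacity on Ability.
; A missing pawn or failed cast only prints a message.
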(event `self.ReceiveBeginPlay`
  (`AbilityComponent.AddAbility` (`self.Ability`) "/Game/Blueprints/Abilities/DA_Flame.DA_Flame") ; TODO: REMOVE (TEST ONLY)
  (`AbilityComponent.AddAbility` (`self.Ability`) "/Game/Blueprints/Abilities/DA_SmallHeal.DA_SmallHeal") ; TODO: REMOVE (TEST ONLY)
  (`AbilityComponent.AddAbility` (`self.Ability`) "/Game/Blueprints/Abilities/DA_Light.DA_Light") ; TODO: REMOVE (TEST ONLY)
  (`AbilityComponent.AddAbility` (`self.Ability`) "/Game/Blueprints/Abilities/DA_StrengthBoost.DA_StrengthBoost") ; TODO: REMOVE (TEST ONLY)
  (`self.GetPawnFromInstance`))

(event `self.ReceiveTick`
  (params (DeltaSeconds :type "Float (single-precision)")))

(fn `GetPawnFromInstance`
  (bind _asflorinstance (cast `/Game/Blueprints/Florinstance` (`GameplayStatics.GetGameInstance`))
    (:`then`
      (bind _has (`/Game/Blueprints/Florinstance.HasPawn` _asflorinstance))
      (if _has
        (`self.RestorePawn` _asflorinstance)
        (else
          (`KismetSystemLibrary.PrintString` "No pawn stored"))))
    (:`CastFailed`
      (`KismetSystemLibrary.PrintString` "game instance cast fail (TBPawn)"))))

(fn `RestorePawn`
  (params (gameInst :type "/Game/Blueprints/Florinstance Object Reference"))
  (bind _healthstatus (`self.HealthStatus`))
  (bind (_playh _playa _playp _playc) (`/Game/Blueprints/Florinstance.GetPawn` gameInst))
  (`HealthStatusComponent.SetCurrentHealth` _healthstatus (`|GetArrayItem` _playh))
  (`HealthStatusComponent.SetMaxHealth` _healthstatus (`|GetArrayItem` _playh 1))
  (`AbilityComponent.SetAbilityArray` (`self.Ability`) _playa)
  (`AbilityComponent.SetCurrentPower` (`self.Ability`) (`|GetArrayItem` _playp))
  (`AbilityComponent.SetMaxPower` (`self.Ability`) (`|GetArrayItem` _playp 1))
  (`AbilityComponent.SetPowerRegenRate` (`self.Ability`) (`|GetArrayItem` _playp 2))
  (`AbilityComponent.SetMaxCapacity` (`self.Ability`) _playc))

(fn `UserConstructionScript`)