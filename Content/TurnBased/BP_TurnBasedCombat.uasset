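; BP_TurnBasedCombat is a turn-based combat Blueprint that so far only implements enemy spawning.
; SpawnCombatants spawns BP_TBEnemy actors in an evenly spaced row along Y, choosing the start position from the enemy count, and passes each the given EnemyType.
; The count is hardcoded to one, with a random-count node left unused and the idle animation call disconnected.
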(event `self.ReceiveBeginPlay`)

(fn `SpawnCombatants`
  (params (enemyType :type "Enemy Object Reference"))
  (locals (numEnemies :type Integer :default 0) (index :type Integer) (spawnPoint :type "Transform Structure") (yPos :type "Float (double-precision)"))
  (bind _output_get (set `local.numEnemies` 1))
  (switch `int` _output_get
    (:`1`
      (set `local.yPos` 700.0))
    (:`2`
      (set `local.yPos` 500.0))
    (:`3`
      (set `local.yPos` 400.0))
    (:`4`
      (set `local.yPos` 300.0)))
  (set `local.spawnPoint` (`KismetMathLibrary.MakeTransform` (`KismetMathLibrary.MakeVector` 75.0 (`local.yPos`)) (struct :`Yaw` 90.0)))
  (while (< (`local.index`) (`local.numEnemies`))
    (bind _returnvalue (`|SpawnActorFromClass` "/Game/TurnBased/BP_TBEnemy.BP_TBEnemy_C" (`local.spawnPoint`) "Undefined" "OverrideRootScale" null null))
    (set `local.yPos` (+ (`local.yPos`) 200.0))
    (set `local.spawnPoint` (`KismetMathLibrary.MakeTransform` (`KismetMathLibrary.MakeVector` 75.0 (`local.yPos`)) (struct :`Yaw` 90.0)))
    (`/Game/TurnBased/BP_TBEnemy.SetEnemyType` _returnvalue enemyType)
    (set `local.index` (+ (`local.index`) 1))))

(fn `UserConstructionScript`)