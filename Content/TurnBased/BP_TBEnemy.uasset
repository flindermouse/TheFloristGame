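; Turn-based enemy Blueprint configured at runtime from an enemy type struct.
; SetEnemyType scales base damage, max health and ability capacity by the type's stats, refills health, then applies its mesh, name text and abilities.
; GetRewards adds at least one random reward from the type's list, possibly repeating and never the last entry when several exist.
; Its debug print re-rolls the random index, so printed names can differ from granted rewards.
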(event `self.ReceiveBeginPlay`)

(event `self.ReceiveTick`
  (params (DeltaSeconds :type "Float (single-precision)")))

(fn `GetRewards`
  (returns (NewParam :type "Array of Item Object Reference"))
  (locals (index :type Integer) (numRewards :type Integer :default 0) (rewards :type "Array of Item Object Reference"))
  (bind _rewards (`Enemy.rewards` (`self.enemyType`)))
  (bind _returnvalue (`KismetArrayLibrary.Array_Length` _rewards))
  (bind _output (`|GetArrayItem` _rewards (`KismetMathLibrary.RandomInteger` (- _returnvalue 1))))
  (bind _output_get (set `local.numRewards` (`KismetMathLibrary.RandomInteger` _returnvalue)))
  (if (== _output_get 0)
    (set `local.numRewards` 1))
  (bind _output_get_2 (set `local.index` 0))
  (while (< _output_get_2 (`local.numRewards`))
    (`KismetArrayLibrary.Array_Add` (`local.rewards`) _output)
    (set `local.index` (+ (`local.index`) 1))
    (`KismetSystemLibrary.PrintString` (`KismetStringLibrary.Conv_NameToString` (`Item.name` _output))))
  (return (`local.rewards`)))

(fn `SetEnemyType`
  (params (type :type "Enemy Object Reference"))
  (bind _returnvalue (`HealthStatusComponent.GetMaxHealth` (`self.HealthStatus`)))
  (set `self.enemyType` type)
  (`self.SetBaseDamage` (* (`Enemy.strength` (`self.enemyType`)) (`self.GetBaseDamage`)))
  (`HealthStatusComponent.SetMaxHealth` (`self.HealthStatus`) (* (`Enemy.endurance` (`self.enemyType`)) _returnvalue))
  (`HealthStatusComponent.SetCurrentHealth` (`self.HealthStatus`) _returnvalue)
  (`HealthStatusComponent.SetCurrentHealth` (`self.HealthStatus`) _returnvalue)
  (`AbilityComponent.SetMaxCapacity` (`self.Ability`) (`KismetMathLibrary.FTrunc` (* (`Enemy.experience` (`self.enemyType`)) (`AbilityComponent.GetMaxPower` (`self.Ability`)))))
  (`SkinnedMeshComponent.SetSkinnedAssetAndUpdate` (`self.SkeletalMesh`) (`Enemy.mesh` (`self.enemyType`)) true)
  (`TextRenderComponent.K2_SetText` (`self.TextRender`) (`KismetTextLibrary.Conv_StringToText` (`Enemy.name` (`self.enemyType`))))
  (for _array_element (`Enemy.abilities` (`self.enemyType`))
    (`AbilityComponent.AddAbility` (`self.Ability`) _array_element)))

(fn `UserConstructionScript`)